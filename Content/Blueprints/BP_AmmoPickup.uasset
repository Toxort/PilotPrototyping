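; BP_AmmoPickup is an ammo pickup actor that hands its AmmoType to the player's current weapon.
; Every Tick it casts player 0's character to BP_MainCharacter and polls its EPressed flag, with no overlap or distance check.
; While the flag is set, it destroys itself, then writes AmmoType into the Inventory of CurrentShotWeapon.
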(event `self.ReceiveTick`
  (params (DeltaSeconds :type "Float (single-precision)"))
  (bind __ (`self.-`))
  (bind _asbp_main_character (cast `/Game/Blueprints/BP_MainCharacter` (`GameplayStatics.GetPlayerCharacter` 0)))
  (bind _output_get (set `self.As BP Main Character` _asbp_main_character))
  (if (`MainCharacter.bEPressed` _output_get)
    (`self.K2_DestroyActor`)
    (set `Weapon.Inventory` (`|MakeArray` (`self.AmmoType`) __ __) (`MainCharacter.CurrentShotWeapon` (`self.As BP Main Character`)))))

(fn `UserConstructionScript`)