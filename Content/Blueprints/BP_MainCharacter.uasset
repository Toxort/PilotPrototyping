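; Main character Blueprint that handles right-mouse aiming and left-click throwing, gated by a side-character cooldown.
; Tick rotates the throw transform toward the mouse, deriving pitch from cursor distance.
; While aiming, a runtime spline follows a predicted projectile path, with a BP_EndPoint actor marking the impact.
; Throwing clears the preview, then after a short delay spawns ThrowableTest using a suggested toss velocity toward the mouse, calculated separately from the preview.
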(event `self.ReceiveBeginPlay`)

(event `self.ReceiveTick`
  (params (DeltaSeconds :type "Float (single-precision)"))
  (bind (_yrotation_roll _yrotation_pitch _yrotation_yaw) (`KismetMathLibrary.BreakRotator` (`self.YRotation`)))
  (bind _returnvalue (+ (`SceneComponent.K2_GetComponentLocation` (`self.ThrowTransform`)) (+ (`self.SideCharacterSpawnPoint`) (0.0 0.0 75.0))))
  (bind _returnvalue_2 (`self.GetMouseDirection` (+ (`self.K2_GetActorLocation`) (`self.SideCharacterSpawnPoint`))))
  (`SceneComponent.K2_SetRelativeRotation` (`self.ThrowTransformRotated`) _returnvalue_2 false false)
  (set `self.YRotation` _returnvalue_2)
  (set `self.YRotation` (`KismetMathLibrary.MakeRotator` _yrotation_roll (/ (`KismetMathLibrary.FClamp` (- (`self.distanceMouseToPlayer`) 1750.0) -2000.0 2000.0) 20.0) _yrotation_yaw))
  (`|ExecutionSequence`
    (:`then_0`
      (`self.DrawPredictionSpline`)
      (if (`self.bRightMouseButtonPressed`)
        (`/Engine/EditorBlueprintResources/StandardMacros.DoOnce` false :!label _label
          (:`Completed`
            (`self.CreatePredictionSpline`)
            (set `self.isAiming` true)
            (goto _label_2 :!via `Reset`)))
        (else
          (`/Engine/EditorBlueprintResources/StandardMacros.DoOnce` false :!label _label_2
            (:`Completed`
              (`self.DestroyPredicionSpline`)
              (set `self.isAiming` false)
              (goto _label :!via `Reset`))))))
    (:`then_1`
      (if (`self.bLeftClickedPressed`)
        (if (not (`self.bSideCharacterOnCooldown`))
          (if (`self.isAiming`)
            (`self.SideCharacterThrow`)
            (`self.DestroyPredicionSpline`)
            (bind _returnvalue_3 (`self.GetMousePosition`))
            (bind _tossvelocity (`GameplayStatics.BlueprintSuggestProjectileVelocity` _returnvalue _returnvalue_3 (`self.ThrowSpeed`) 0.0 "DoNotTrace"))
            (`KismetSystemLibrary.Delay` 0.2)
            (`|SpawnActorFromClass` "/Game/Blueprints/ThrowableTest.ThrowableTest_C" (`KismetMathLibrary.Conv_VectorToTransform` _returnvalue) "Undefined" "OverrideRootScale" null _tossvelocity null)))))))

(fn `CreatePredictionSpline`
  (`/Engine/EditorBlueprintResources/StandardMacros.DoOnce` false
    (:`Completed`
      (bind _returnvalue (`AddComponent|NODE_AddSplineComponent-0`))
      (set `self.PredictionSpline_0` _returnvalue)
      (bind _returnvalue_2 (`|SpawnActorFromClass` "/Game/Meshes/PredictionPath/BP_EndPoint.BP_EndPoint_C" (`KismetMathLibrary.MakeTransform` (0.0 0.0 0.0)) "Undefined" "OverrideRootScale" null null))
      (bind _output_get (set `self.PredictionEndPoint` _returnvalue_2))
      (`self.SetActorHiddenInGame` _output_get true))))

(fn `DestroyPredicionMeshes`)

(fn `DestroyPredicionSpline`
  (bind _predictionspline_0 (`self.PredictionSpline_0`)
    (:`then`
      (`ActorComponent.K2_DestroyComponent` _predictionspline_0)
      (set `self.PredictionSpline_0` null)
      (`self.DestroyPredicionMeshes`)
      (`self.K2_DestroyActor` (`self.PredictionEndPoint`))
      (set `self.PredictionEndPoint` null)
      (set `self.isAiming` false))
    (:`else`)))

(fn `DrawPredictionSpline`
  (bind _predictionendpoint (`self.PredictionEndPoint`))
  (`/Engine/EditorBlueprintResources/StandardMacros.DoOnce` false
    (:`Completed`
      (`self.PredictionSplineValid`
        (:`Is Valid`
          (`|ExecutionSequence`
            (:`then_0`
              (bind (_outhit _outpathpositions _outlasttracedestination _returnvalue) (`GameplayStatics.Blueprint_PredictProjectilePath_ByTraceChannel` (+ (`self.K2_GetActorLocation`) (`self.SideCharacterThrowPoint`)) (+ (* (`self.YRotation`) (`self.ThrowSpeed`)) (`self.SideCharacterSpawnPoint`)) false 25.0 "ECC_WorldDynamic" false (`|MakeArray` self :!type "Actor Object Reference") "None" 0.1 15.0 1.0))
              (if _returnvalue
                (`self.SetActorHiddenInGame` _predictionendpoint false)
                (`self.K2_SetActorLocation` _predictionendpoint (`.ImpactPoint` (`GameplayStatics.BreakHitResult` _outhit)) false true)
                (else
                  (`self.SetActorHiddenInGame` (`self.PredictionEndPoint`) true)))
              (`SplineComponent.SetSplinePoints` (`self.PredictionSpline_0`) _outpathpositions "World" true)
              (`self.DestroyPredicionMeshes`))))))))

(fn `UserConstructionScript`)